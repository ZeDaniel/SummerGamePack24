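; BP_BallemGameInstance is the game instance that handles progression through an ordered list of levels.
; SwitchLevel finds the current level's name in LevelList and opens the following entry by name.
; On the last level it instead plays an explosion sound at the player pawn, waits briefly and quits the game.
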(event Custom|SwitchLevel
  (bind _levellist (Variables|Default|GetLevelList))
  (bind _returnvalue (Game|GetCurrentLevelName true))
  (for (_array_element _array_index) _levellist
    (if (Utilities|Enum|Equal(Enum) _array_element _returnvalue)
      (if (== _array_index (- (Utilities|Array|Length _levellist) 1))
        (Audio|PlaySoundatLocation "/Game/Sounds/medium-explosion-40472.medium-explosion-40472" (Transformation|GetActorLocation (Game|Player|GetPlayerPawn 0)) "0, 0, 0" 1.0 1.0 0.0 0 0 0 0)
        (Utilities|FlowControl|Delay 1.0)
        (Game|QuitGame 0 "Quit" false)
        (else
          (Game|OpenLevel(byName) (Utilities|String|StringToName (Utilities|Array|Get(acopy) (Variables|Default|GetLevelList) (+ _array_index 1)))))))))