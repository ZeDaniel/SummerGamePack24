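; Game mode for The Punch that manages the UI of its microgame flow and forces a windowed resolution on BeginPlay.
; Events create and show the microgame, transition and start-transition widgets.
; ClearWidgets removes any launch, transition and start-transition widgets, and runs before the transition phase widget is shown.
; RestartGame reloads the current level by name.
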(event Custom|ClearWidgets
  (bind _foundwidgets (Widget|GetAllWidgetsOfClass "/Game/Blueprints/Widgets/BP_TransitionPhaseWidget.BP_TransitionPhaseWidget_C" true))
  (for _array_element _foundwidgets
    (Widget|RemovefromParent _array_element))
  (bind _foundwidgets_2 (Widget|GetAllWidgetsOfClass "/Game/Blueprints/Widgets/BP_StartTransitionPhaseWidget.BP_StartTransitionPhaseWidget_C" true))
  (for _array_element_2 _foundwidgets_2
    (Widget|RemovefromParent _array_element_2))
  (bind _foundwidgets_3 (Widget|GetAllWidgetsOfClass "/Game/Blueprints/Widgets/BP_LaunchGameWidget.BP_LaunchGameWidget_C" true))
  (for _array_element_3 _foundwidgets_3
    (Widget|RemovefromParent _array_element_3)))

(event EventBeginPlay
  (bind _returnvalue (Settings|GetGameUserSettings))
  (Class|GameUserSettings|SetScreenResolution _returnvalue (Variables|Default|GetResolution))
  (Class|GameUserSettings|SetFullscreenMode _returnvalue "Windowed")
  (Class|GameUserSettings|ApplySettings _returnvalue true))

(event EventTick
  (params (DeltaSeconds :type Float%20%28single-precision%29)))

(event EventRestartGame
  (bind _returnvalue (Game|GetCurrentLevelName true))
  (Game|OpenLevel(byName) (Utilities|String|StringToName _returnvalue)))

(event EventRunStartTransitionPhaseUI
  (bind _returnvalue (UserInterface|CreateWidget "/Game/Blueprints/Widgets/BP_StartTransitionPhaseWidget.BP_StartTransitionPhaseWidget_C"))
  (UserInterface|Viewport|AddtoViewport _returnvalue 0))

(event EventRunTransitionPhaseUI
  (CallFunction|ClearWidgets)
  (bind _returnvalue (UserInterface|CreateWidget "/Game/Blueprints/Widgets/BP_TransitionPhaseWidget.BP_TransitionPhaseWidget_C"))
  (UserInterface|Viewport|AddtoViewport _returnvalue 0))

(event EventRunMicroGameUI
  (bind _returnvalue (UserInterface|CreateWidget "/Game/Blueprints/Widgets/BP_MicroGameWidget.BP_MicroGameWidget_C"))
  (UserInterface|Viewport|AddtoViewport _returnvalue 0))

(fn ConstructionScript)