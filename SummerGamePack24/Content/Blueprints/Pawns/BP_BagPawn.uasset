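; BP_BagPawn is a pawn Blueprint whose graph drives a speed-based camera zoom on its spring arm.
; BeginPlay caches the spring arm's initial length as the base distance.
; Each Tick scales that base by a clamped square root of the pawn's speed and eases the arm toward it with FInterpTo, pulling in when slow and stretching out when fast.
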(event EventBeginPlay
  (Variables|Default|SetBaseTargetArmLength (Variables|/Script/Engine.SpringArmComponent|GetTargetArmLength (Variables|Default|GetSpringArmComp))))

(event Collision|EventActorBeginOverlap
  (params (OtherActor :type Actor%20Object%20Reference)))

(event EventTick
  (params (DeltaSeconds :type Float%20%28single-precision%29))
  (Variables|/Script/Engine.SpringArmComponent|SetTargetArmLength (Variables|Default|GetSpringArmComp) (Math|Interpolation|FInterpTo (Variables|/Script/Engine.SpringArmComponent|GetTargetArmLength (Variables|Default|GetSpringArmComp)) (* (Math|Float|Clamp(Float) (/ (Math|Float|Sqrt (Math|Vector|VectorLength (Transformation|GetVelocity))) 3e+01) 0.5 3.5) (Variables|Default|GetBaseTargetArmLength)) DeltaSeconds 1.2)))

(fn ConstructionScript)