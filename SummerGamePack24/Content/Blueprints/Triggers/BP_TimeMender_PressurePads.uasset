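; BP_TimeMender_PressurePads is a time mender trigger that attempts to mend once all of its registered pressure pads are activated.
; Pads are added to an array through the AddPressurePad event.
; While active, it polls the array every Tick, skips invalid entries and stops at the first inactive pad.
; If none is inactive, it calls AttemptToMend and, on success, activates the assigned teleport gate.
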(event Custom|AddPressurePad
  (params (NewPressurePad :type BP%20Character%20Trigger%20Object%20Reference%20%28by%20ref%29))
  (Utilities|Array|Add (Variables|TimeSplit|GetPressurePadArray) NewPressurePad))

(event EventBeginPlay)

(event Collision|EventActorBeginOverlap
  (params (OtherActor :type Actor%20Object%20Reference)))

(event EventTick
  (params (DeltaSeconds :type Float%20%28single-precision%29))
  (bind _teleportgatetoactivate (Variables|TimeMend|GetTeleportGateToActivate))
  (if (Variables|Default|GetIsActive)
    (Variables|TimeMend|SetShouldMend true)
    (bind _array_element (Utilities|Array|ForEachLoopwithBreak (Variables|TimeSplit|GetPressurePadArray) :!label _label)
      (:LoopBody
        (if (Utilities|IsValid _array_element)
          (if (not (Variables|/Game/Blueprints/Triggers/BP_CharacterTrigger.BP_CharacterTrigger_C|GetIsActivated _array_element))
            (Variables|TimeMend|SetShouldMend false)
            (goto _label Break))))
      (:Completed
        (if (Variables|TimeMend|GetShouldMend)
          (bind _returnvalue (Class|TimeMender|AttempttoMend))
          (if _returnvalue
            (if (Utilities|IsValid _teleportgatetoactivate)
              (Default|ActivateGate _teleportgatetoactivate))))))))

(fn ConstructionScript)