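; Decoherence clone character variant that walks on the ceiling under inverted gravity.
; BeginPlay points the movement component's gravity straight up after running the parent logic.
; Its move-input override negates X and derives right and forward directions from the actor's gravity-relative rotation, keeping movement aligned to the flipped frame.
; Look input passes through unchanged.
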(event EventBeginPlay
  (|CallParentFunction)
  (Class|CharacterMovementComponent|SetGravityDirection (Variables|Character|GetCharacterMovement) (Math|Vector|MakeVector 0.0 0.0 1.0)))

(event Collision|EventActorBeginOverlap
  (params (OtherActor :type Actor%20Object%20Reference))
  (|CallParentFunction OtherActor) ; This node is disabled and will not be called.\nDrag off pins to build functionality.
)

(event EventTick
  (params (DeltaSeconds :type Float%20%28single-precision%29))
  (|CallParentFunction DeltaSeconds) ; This node is disabled and will not be called.\nDrag off pins to build functionality.
)

(event EventAlterMoveInput
  (params (Value :type Input%20Action%20Value%20Structure%20%28by%20ref%29))
  (bind (_x _y _z) (Class|EnhancedInputLibrary|BreakInputActionValue Value))
  (bind _returnvalue (Transformation|GetActorRotation))
  (bind _charactermovement (Variables|Character|GetCharacterMovement))
  (bind _charactermovement_2 (Variables|Character|GetCharacterMovement))
  (bind _gravitydirection (Variables|/Script/Engine.CharacterMovementComponent|GetGravityDirection _charactermovement))
  (bind _gravitydirection_2 (Variables|/Script/Engine.CharacterMovementComponent|GetGravityDirection _charactermovement_2))
  (bind _returnvalue_2 (Class|GravityController|GetGravityRelativeRotation _returnvalue _gravitydirection_2))
  (Variables|Default|SetAlteredInput (Class|EnhancedInputLibrary|MakeInputActionValueOfType (* _x -1.0) _y _z "Axis2D"))
  (Variables|Default|SetLRWorldDirection (Math|Vector|GetRightVector (Class|GravityController|GetGravityWorldRotation (Math|Rotator|MakeRotator (.roll _returnvalue_2) 0.0 (.yaw _returnvalue_2)) _gravitydirection_2)))
  (Variables|Default|SetFBWorldDirection (Math|Vector|GetForwardVector (Class|GravityController|GetGravityWorldRotation (Math|Rotator|MakeRotator 0.0 0.0 (.yaw (Class|GravityController|GetGravityRelativeRotation (Transformation|GetActorRotation) _gravitydirection))) _gravitydirection))))

(event EventAlterLookInput
  (params (Value :type Input%20Action%20Value%20Structure%20%28by%20ref%29))
  (Variables|Default|SetAlteredInput Value))

(fn ConstructionScript
  (|CallParentFunction))