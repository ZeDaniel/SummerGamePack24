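; BP_SGP24GameMode is the SGP24 game mode that handles level startup, pausing, restarting and developer commentary visibility.
; BeginPlay applies the default resolution in fullscreen, adds the player HUD, sets game-only input and toggles commentary when the game instance has it disabled.
; Pause and unpause events add or remove the pause widget while switching cursor, input mode and paused state.
; Commentary toggling flips root component visibility on actors tagged DevCommentary.
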(event Custom|ToggleCommentaryVisibility
  ;[1 1 1] Toggle visibility of extra dev commentary
  (bind _outactors (Actor|GetAllActorswithTag "DevCommentary"))
  (Utilities|Casting|CastToBP_SGP24GameInstance (Game|GetGameInstance))
  (for _array_element _outactors
    (Rendering|ToggleVisibility (Variables|/Script/Engine.Actor|GetRootComponent _array_element) true)))

(event Custom|PauseGame
  (bind _returnvalue (Game|GetPlayerController 0))
  ;[1 1 1] Pause and UnPause
  (bind _returnvalue_2 (UserInterface|CreateWidget "/Game/Widgets/BP_SGP24_PauseWidget.BP_SGP24_PauseWidget_C"))
  (UserInterface|Viewport|AddtoViewport _returnvalue_2 0)
  (Variables|/Script/Engine.PlayerController|SetbShowMouseCursor _returnvalue true)
  (Variables|Default|SetGamePaused true)
  (Input|SetInputModeGameandUI _returnvalue _returnvalue_2 "DoNotLock" false false)
  (Game|SetGamePaused true))

(event Custom|UnPauseGame
  (bind _returnvalue (Game|GetPlayerController 0))
  ;[1 1 1] Pause and UnPause
  (Widget|RemovefromParent (stale Custom|PauseGame _returnvalue_2))
  (Variables|/Script/Engine.PlayerController|SetbShowMouseCursor _returnvalue false)
  (Variables|Default|SetGamePaused false)
  (Input|SetInputModeGameOnly _returnvalue false)
  (Game|SetGamePaused false))

(event Custom|RestartLevel
  ;[1 1 1] Restart Level
  (bind _returnvalue (Game|GetCurrentLevelName true))
  (Game|OpenLevel(byName) (Utilities|String|StringToName _returnvalue)))

(event EventBeginPlay
  ;[1 1 1] Set screen resolution and windowed setting
  (bind _returnvalue (Settings|GetGameUserSettings))
  (bind _returnvalue_2 (Class|GameUserSettings|GetDefaultResolution))
  (Class|GameUserSettings|SetScreenResolution _returnvalue _returnvalue_2)
  (Class|GameUserSettings|SetFullscreenMode _returnvalue "Fullscreen")
  (Class|GameUserSettings|ApplySettings _returnvalue true)
  ;[1 1 1] Player Input and Hud
  (bind _returnvalue_3 (UserInterface|CreateWidget "/Game/Widgets/BP_SGP24_PlayerHud.BP_SGP24_PlayerHud_C"))
  (UserInterface|Viewport|AddtoViewport _returnvalue_3 0)
  (Input|SetInputModeGameOnly (Game|GetPlayerController 0) false)
  (bind _asbp_sgp24game_instance (Utilities|Casting|CastToBP_SGP24GameInstance (Game|GetGameInstance)))
  (if (not (Variables|/Game/SumGamePack/GameMode/BP_SGP24GameInstance.BP_SGP24GameInstance_C|GetCommentaryEnabled _asbp_sgp24game_instance))
    (CallFunction|ToggleCommentaryVisibility)))

(event EventTick
  (params (DeltaSeconds :type Float%20%28single-precision%29)))

(fn ConstructionScript)