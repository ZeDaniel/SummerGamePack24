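; Game instance for SumGamePack that carries score and level progression for the Roller game and level switching for Ballem.
; Reaching the target score ends the Roller game mode, then WinGame advances the level after a delay.
; Past the last level, it shows an end widget and adds a restart input mapping.
; SwitchLevel steps through a level list, returning to the hub world with an explosion sound after the last.
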(event Custom|SwitchLevel
  (bind _levellist (Variables|Default|GetLevelList))
  ;[1 1 1] Ballem Instance code
  (bind _returnvalue (Game|GetCurrentLevelName true))
  (for (_array_element _array_index) _levellist
    (if (Utilities|Enum|Equal(Enum) _array_element _returnvalue)
      (if (== _array_index (- (Utilities|Array|Length _levellist) 1))
        (Audio|PlaySoundatLocation "/Game/Sounds/medium-explosion-40472.medium-explosion-40472" (Transformation|GetActorLocation (Game|Player|GetPlayerPawn 0)) "0, 0, 0" 1.0 1.0 0.0 0 0 0 0)
        (Utilities|FlowControl|Delay 1.0)
        (Game|OpenLevel(byObjectReference) "/Game/SumGamePack/Maps/SumGamePack_HubWorld.SumGamePack_HubWorld")
        (else
          (Game|OpenLevel(byName) (Utilities|String|StringToName (Utilities|Array|Get(acopy) (Variables|Default|GetLevelList) (+ _array_index 1)))))))))

(event Custom|RestartGame
  ;[1 1 1] Roller Instance code
  ;;[1 1 1] Restart Game
  (Variables|Default|SetCurrentScore 0)
  (Variables|Default|SetCurrentLevel 0)
  (Game|OpenLevel(byObjectReference) "/Game/Sub-Games/01_Roller/Roller/Maps/Roller_Level01.Roller_Level01"))

(event Custom|SetTargetScore
  (params (TargetScore :type Integer))
  ;[1 1 1] Roller Instance code
  ;;[1 1 1] Public function to set target score
  (Variables|Default|SetTargetScore TargetScore))

(event Custom|IncreaseScore
  ;[1 1 1] Roller Instance code
  ;;[1 1 1] Increase score and check for win condition
  (Variables|Default|SetCurrentScore (+ (Variables|Default|GetCurrentScore) 1))
  (if (== (Variables|Default|GetCurrentScore) (Variables|Default|GetTargetScore))
    (bind _asbp_roller_game_mode (Utilities|Casting|CastToBP_RollerGameMode (Game|GetGameMode)))
    (Default|EndGame _asbp_roller_game_mode)
    (CallFunction|WinGame)))

(event Custom|WinGame
  ;[1 1 1] Roller Instance code
  ;;[1 1 1] Win game and transition levels
  (Variables|Default|SetCurrentScore 0)
  (Variables|Default|SetCurrentLevel (+ (Variables|Default|GetCurrentLevel) 1))
  (Utilities|FlowControl|Delay 3.0)
  (switch int (Variables|Default|GetCurrentLevel)
    (:Default
      ;;[1 1 1] Handle End of Game
      (bind _returnvalue (UserInterface|CreateWidget "/Game/Sub-Games/01_Roller/Roller/Blueprints/BP_EndWidget.BP_EndWidget_C"))
      (UserInterface|Viewport|AddtoViewport _returnvalue 0)
      (bind _asbp_level_controller (Utilities|Casting|CastToBP_LevelController (Game|GetPlayerController 0)))
      (Input|AddMappingContext (PlayerController|LocalPlayerSubsystems|GetEnhancedInputLocalPlayerSubsystem _asbp_level_controller) "/Game/Sub-Games/01_Roller/Roller/Input/RestartController.RestartController" 0 "(bIgnoreAllPressedKeysUntilRelease=True,bForceImmediately=False,bNotifyUserSettings=False)"))
    (:0
      (Development|PrintString "WHAT? HOW?"))
    (:1
      (Game|OpenLevel(byObjectReference) "/Game/Sub-Games/01_Roller/Roller/Maps/Roller_Level02.Roller_Level02"))
    (:2
      (Game|OpenLevel(byObjectReference) "/Game/Sub-Games/01_Roller/Roller/Maps/Roller_Level03.Roller_Level03"))
    (:3
      (Game|OpenLevel(byObjectReference) "/Game/Sub-Games/01_Roller/Roller/Maps/Roller_Level04.Roller_Level04"))
    (:4
      (Game|OpenLevel(byObjectReference) "/Game/Sub-Games/01_Roller/Roller/Maps/Roller_Level05.Roller_Level05"))))