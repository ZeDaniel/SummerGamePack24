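; Game mode Blueprint for the Safety sub-game that handles its controls display, pausing and level restarts.
; On BeginPlay it creates and shows a controls widget.
; Pause and unpause events add or remove a pause menu widget, toggle the mouse cursor, and set both a GamePaused flag and the engine pause state.
; The restart event reopens the current level by name.
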(event Custom|PauseGame
  (bind _returnvalue (UserInterface|CreateWidget "/Game/Widgets/04_Safety/Safety_BP_PauseWidget.Safety_BP_PauseWidget_C"))
  (UserInterface|Viewport|AddtoViewport _returnvalue 0)
  (Variables|/Script/Engine.PlayerController|SetbShowMouseCursor (Game|GetPlayerController 0) true)
  (Variables|Default|SetGamePaused true)
  (Game|SetGamePaused true))

(event Custom|UnPauseGame
  (Widget|RemovefromParent (stale Custom|PauseGame _returnvalue))
  (Variables|/Script/Engine.PlayerController|SetbShowMouseCursor (Game|GetPlayerController 0) false)
  (Variables|Default|SetGamePaused false)
  (Game|SetGamePaused false))

(event Custom|RestartLevel
  (bind _returnvalue (Game|GetCurrentLevelName true))
  (Game|OpenLevel(byName) (Utilities|String|StringToName _returnvalue)))

(event EventBeginPlay
  (bind _returnvalue (UserInterface|CreateWidget "/Game/Widgets/04_Safety/Safety_BP_ControlsWidget.Safety_BP_ControlsWidget_C"))
  (UserInterface|Viewport|AddtoViewport _returnvalue 0))

(event EventTick
  (params (DeltaSeconds :type Float%20%28single-precision%29)))

(fn ConstructionScript)