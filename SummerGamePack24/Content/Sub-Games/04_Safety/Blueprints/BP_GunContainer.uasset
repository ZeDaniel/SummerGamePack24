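; BP_GunContainer is an interactable gun container in the Safety sub-game that can be opened only by a character tagged SAFE.
; Overlap by BP_SafetyCharacter shows BP_GunPopupWidget and enables input if the tag is present, and leaving reverses both.
; A valid interaction removes the SAFE tag and popup, then destroys the window, mesh and text components.
; Otherwise, interacting triggers the widget's rejection text.
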(event OnInteract(Interactable)
  (if (Variables|Default|GetAcceptsInput)
    (Utilities|Array|RemoveItem (Variables|/Script/Engine.Actor|GetTags (stale Collision|EventActorBeginOverlap _asbp_safety_character)) "SAFE")
    (Widget|RemovefromParent (stale Collision|EventActorBeginOverlap _returnvalue))
    (Components|DestroyComponent (Variables|Default|GetSM_Window_HP))
    (else
      (Default|ActivateRejectText (stale Collision|EventActorBeginOverlap _returnvalue)))))

(event EventBeginPlay)

(event Collision|EventActorBeginOverlap
  (params (OtherActor :type Actor%20Object%20Reference))
  (bind _asbp_safety_character (Utilities|Casting|CastToBP_SafetyCharacter OtherActor))
  (bind _returnvalue (UserInterface|CreateWidget "/Game/Widgets/04_Safety/BP_GunPopupWidget.BP_GunPopupWidget_C"))
  (UserInterface|Viewport|AddtoViewport _returnvalue 0)
  (if (Actor|ActorHasTag _asbp_safety_character "SAFE")
    (Variables|Default|SetAcceptsInput true)))

(event EventTick
  (params (DeltaSeconds :type Float%20%28single-precision%29)))

(event Collision|EventActorEndOverlap
  (params (OtherActor :type Actor%20Object%20Reference))
  (Utilities|Casting|CastToBP_SafetyCharacter OtherActor)
  (Variables|Default|SetAcceptsInput false)
  (Widget|RemovefromParent (stale Collision|EventActorBeginOverlap _returnvalue)))

(fn ConstructionScript)