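; BP_NewNonPickUp_Item_PowerUp is a power-up item for the Safety sub-game that permanently boosts the movement of the character who picks it up.
; When its Safety_TP_PickUp component fires OnPickUp, it casts the picker to BP_SafetyCharacter and gets its CharacterMovementComponent.
; It then adds configurable amounts to max walk speed, jump velocity, air control and max fly speed, with no timer or revert.
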(event OnPickUp(Safety_TP_PickUp)
  (params (PickUpCharacter :type Safety%20Character%20Object%20Reference))
  (bind _asbp_safety_character (Utilities|Casting|CastToBP_SafetyCharacter PickUpCharacter))
  (bind _ascharacter_movement_component (Utilities|Casting|CastToCharacterMovementComponent (Pawn|GetMovementComponent _asbp_safety_character)))
  (Variables|/Script/Engine.CharacterMovementComponent|SetMaxWalkSpeed _ascharacter_movement_component (+ (Variables|/Script/Engine.CharacterMovementComponent|GetMaxWalkSpeed _ascharacter_movement_component) (Variables|Default|GetSpeedAdded)))
  (Variables|/Script/Engine.CharacterMovementComponent|SetJumpZVelocity _ascharacter_movement_component (+ (Variables|/Script/Engine.CharacterMovementComponent|GetJumpZVelocity _ascharacter_movement_component) (Variables|Default|GetJumpVelocityAdded)))
  (Variables|/Script/Engine.CharacterMovementComponent|SetAirControl _ascharacter_movement_component (+ (Variables|/Script/Engine.CharacterMovementComponent|GetAirControl _ascharacter_movement_component) (Variables|Default|GetAirControlAdded)))
  (Variables|/Script/Engine.CharacterMovementComponent|SetMaxFlySpeed _ascharacter_movement_component (+ (Variables|/Script/Engine.CharacterMovementComponent|GetMaxFlySpeed _ascharacter_movement_component) (Variables|Default|GetFlyVelocityAdded))))

(event EventBeginPlay
  (|CallParentFunction) ; This node is disabled and will not be called.\nDrag off pins to build functionality.
)

(event Collision|EventActorBeginOverlap
  (params (OtherActor :type Actor%20Object%20Reference))
  (|CallParentFunction OtherActor) ; This node is disabled and will not be called.\nDrag off pins to build functionality.
)

(event EventTick
  (params (DeltaSeconds :type Float%20%28single-precision%29))
  (|CallParentFunction DeltaSeconds) ; This node is disabled and will not be called.\nDrag off pins to build functionality.
)

(fn ConstructionScript
  (|CallParentFunction))