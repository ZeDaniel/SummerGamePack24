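; BP_NewPickUp_Item is a pickup item in the Safety sub-game that the player character can pick up and put down.
; On pickup it calls AttachItem on its Item and, if that succeeds, shrinks to a fifth scale and sets the first-person mesh's AnimBP pose to "Paper".
; On put-down it resets the pose to "Base" but does not restore the scale.
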(event OnPickUp(Safety_TP_PickUp)
  (params (PickUpCharacter :type Safety%20Character%20Object%20Reference))
  (bind _returnvalue (Class|ItemComponent|AttachItem (Variables|Default|GetItem) PickUpCharacter))
  (if _returnvalue
    (CallFunction|Shrink)
    (bind _assafety_first_person_anim_bp (Utilities|Casting|CastToSafety_FirstPerson_AnimBP (Components|SkeletalMesh|GetAnimInstance (Variables|/Script/SummerGamePack24.SafetyCharacter|GetMesh1P PickUpCharacter))))
    (Variables|/Game/FirstPersonArms/Animations/SafetyAnimations/Safety_FirstPerson_AnimBP.Safety_FirstPerson_AnimBP_C|SetPoseClass _assafety_first_person_anim_bp "Paper")))

(event OnPutDown(Safety_TP_PickUp)
  (params (PickUpCharacter :type Safety%20Character%20Object%20Reference))
  (bind _assafety_first_person_anim_bp (Utilities|Casting|CastToSafety_FirstPerson_AnimBP (Components|SkeletalMesh|GetAnimInstance (Variables|/Script/SummerGamePack24.SafetyCharacter|GetMesh1P PickUpCharacter))))
  (Variables|/Game/FirstPersonArms/Animations/SafetyAnimations/Safety_FirstPerson_AnimBP.Safety_FirstPerson_AnimBP_C|SetPoseClass _assafety_first_person_anim_bp "Base"))

(event EventBeginPlay)

(event Collision|EventActorBeginOverlap
  (params (OtherActor :type Actor%20Object%20Reference)))

(event EventTick
  (params (DeltaSeconds :type Float%20%28single-precision%29)))

(fn ConstructionScript)

(fn Shrink
  (Transformation|SetActorScale3D "0.200000,0.200000,0.200000"))