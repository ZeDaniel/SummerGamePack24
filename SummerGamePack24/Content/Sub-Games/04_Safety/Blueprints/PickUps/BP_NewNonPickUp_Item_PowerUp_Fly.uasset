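; Flight power-up item for the Safety sub-game that switches the character who picks it up into flying.
; The Safety_TP_PickUp component's OnPickUp event casts the picker to BP_SafetyCharacter and sets its IsFlying flag.
; It then puts the character movement component in Flying mode with a high braking deceleration.
; Nothing in this Blueprint reverts the flight state.
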(event OnPickUp(Safety_TP_PickUp)
  (params (PickUpCharacter :type Safety%20Character%20Object%20Reference))
  (bind _asbp_safety_character (Utilities|Casting|CastToBP_SafetyCharacter PickUpCharacter))
  (Variables|/Script/SummerGamePack24.SafetyCharacter|SetIsFlying _asbp_safety_character true)
  (bind _ascharacter_movement_component (Utilities|Casting|CastToCharacterMovementComponent (Pawn|GetMovementComponent _asbp_safety_character)))
  (Pawn|Components|CharacterMovement|SetMovementMode _ascharacter_movement_component "MOVE_Flying" 0)
  (Variables|/Script/Engine.CharacterMovementComponent|SetBrakingDecelerationFlying _ascharacter_movement_component 1.5e+04))

(event EventBeginPlay
  (|CallParentFunction) ; This node is disabled and will not be called.\nDrag off pins to build functionality.
)

(event Collision|EventActorBeginOverlap
  (params (OtherActor :type Actor%20Object%20Reference))
  (|CallParentFunction OtherActor) ; This node is disabled and will not be called.\nDrag off pins to build functionality.
)

(event EventTick
  (params (DeltaSeconds :type Float%20%28single-precision%29))
  (|CallParentFunction DeltaSeconds) ; This node is disabled and will not be called.\nDrag off pins to build functionality.
)

(fn ConstructionScript
  (|CallParentFunction))