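; Held-item destruction field for the Safety sub-game that, when its action runs, tags the player SAFE and teleports them to a fixed spot.
; PerformAction overrides the player's location and rotation, then calls DisableInput using the Safety player controller and waits briefly.
; If the player still has the SAFE tag after the delay, it calls EnableInput and adds the clear-screen widget to the viewport.
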(event EventBeginPlay
  (|CallParentFunction) ; This node is disabled and will not be called.\nDrag off pins to build functionality.
)

(event Collision|EventActorBeginOverlap
  (params (OtherActor :type Actor%20Object%20Reference))
  (|CallParentFunction OtherActor) ; This node is disabled and will not be called.\nDrag off pins to build functionality.
)

(event EventTick
  (params (DeltaSeconds :type Float%20%28single-precision%29))
  (|CallParentFunction DeltaSeconds) ; This node is disabled and will not be called.\nDrag off pins to build functionality.
)

(event EventPerformAction
  (bind _returnvalue (Game|GetPlayerCharacter 0))
  (Utilities|Array|Add (Variables|/Script/Engine.Actor|GetTags _returnvalue) "SAFE")
  (Transformation|SetActorLocationAndRotation _returnvalue "680.000000,900.000000,100.000000" "0.000000,180.000000,0.000000")
  (bind _asbp_safety_player_controller (Utilities|Casting|CastToBP_SafetyPlayerController (Pawn|GetController _returnvalue)))
  (Input|DisableInput _asbp_safety_player_controller)
  (Utilities|FlowControl|Delay 3.0)
  (if (Actor|ActorHasTag _returnvalue "SAFE")
    (Input|EnableInput _asbp_safety_player_controller 0)
    (bind _returnvalue_2 (UserInterface|CreateWidget "/Game/Widgets/04_Safety/BP_ClearScreenWidget.BP_ClearScreenWidget_C"))
    (UserInterface|Viewport|AddtoViewport _returnvalue_2 0)))

(fn ConstructionScript
  (|CallParentFunction))