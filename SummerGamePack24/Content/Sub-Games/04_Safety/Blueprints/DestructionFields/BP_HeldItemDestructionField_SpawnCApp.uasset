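; Held-item destruction field variant for the Safety sub-game that spawns a college application pickup when its action runs.
; PerformAction spawns a BP_NewPickUp_Item at a fixed world-axis offset from the field's location.
; It tags the new item's component as "CollegeApp" and "SafeApplication" and applies a gray metal template material.
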(event EventBeginPlay
  (|CallParentFunction) ; This node is disabled and will not be called.\nDrag off pins to build functionality.
)

(event Collision|EventActorBeginOverlap
  (params (OtherActor :type Actor%20Object%20Reference))
  (|CallParentFunction OtherActor) ; This node is disabled and will not be called.\nDrag off pins to build functionality.
)

(event EventTick
  (params (DeltaSeconds :type Float%20%28single-precision%29))
  (|CallParentFunction DeltaSeconds) ; This node is disabled and will not be called.\nDrag off pins to build functionality.
)

(event EventPerformAction
  (bind _returnvalue (Game|SpawnActorfromClass "/Game/Sub-Games/04_Safety/Blueprints/PickUps/BP_NewPickUp_Item.BP_NewPickUp_Item_C" (Math|Transform|MakeTransform (- (.Location (Math|Transform|BreakTransform (Transformation|GetActorTransform))) "1300.000000,0.000000,150.000000")) "Undefined" "MultiplyWithRoot" 0 0))
  (Utilities|Array|Add (Variables|/Script/Engine.ActorComponent|GetComponentTags (Actor|GetComponentbyClass _returnvalue "/Script/SummerGamePack24.ItemComponent")) "CollegeApp")
  (Utilities|Array|Add (Variables|/Script/Engine.ActorComponent|GetComponentTags (Actor|GetComponentbyClass _returnvalue "/Script/SummerGamePack24.ItemComponent")) "SafeApplication")
  (Rendering|Material|SetMaterial (Actor|GetComponentbyClass _returnvalue "/Script/SummerGamePack24.ItemComponent") 0 "/Engine/TemplateResources/MI_Template_BaseGray_02_Metal.MI_Template_BaseGray_02_Metal"))

(fn ConstructionScript
  (|CallParentFunction))