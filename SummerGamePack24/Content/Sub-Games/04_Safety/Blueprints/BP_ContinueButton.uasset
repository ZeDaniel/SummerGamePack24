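; BP_ContinueButton is an interactable in the Safety sub-game that sends the player back to the game pack's hub world.
; Overlap by BP_SafetyCharacter shows a quit widget, and leaving removes it.
; Interacting removes the widget and starts a countdown on Tick, which scales a post-process vector setting down as a screen transition, then opens SumGamePack_HubWorld when time runs out.
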(event OnInteract(Interactable)
  (Variables|Default|SetIsQuitting true)
  (Widget|RemovefromParent (stale Collision|EventActorBeginOverlap _returnvalue)))

(event EventBeginPlay)

(event Collision|EventActorBeginOverlap
  (params (OtherActor :type Actor%20Object%20Reference))
  (Utilities|Casting|CastToBP_SafetyCharacter OtherActor)
  (bind _returnvalue (UserInterface|CreateWidget "/Game/Widgets/04_Safety/BP_QuitWidget.BP_QuitWidget_C"))
  (UserInterface|Viewport|AddtoViewport _returnvalue 0))

(event EventTick
  (params (DeltaSeconds :type Float%20%28single-precision%29))
  (if (Variables|Default|GetIsQuitting)
    (Variables|Default|SetQuitTimer (- (Variables|Default|GetQuitTimer) DeltaSeconds))
    (Variables|/Script/Engine.PostProcessVolume|SetSettings (Variables|Default|GetPostProcessVolume) (Utilities|Struct|MakePostProcessSettings (Math|Vector4|MakeVector4 (/ (Variables|Default|GetQuitTimer) 3.0) (/ (Variables|Default|GetQuitTimer) 3.0) (/ (Variables|Default|GetQuitTimer) 3.0) 0.0)))
    (if (<= (Variables|Default|GetQuitTimer) 0.0)
      (Game|OpenLevel(byObjectReference) "/Game/SumGamePack/Maps/SumGamePack_HubWorld.SumGamePack_HubWorld"))))

(event Collision|EventActorEndOverlap
  (params (OtherActor :type Actor%20Object%20Reference))
  (Utilities|Casting|CastToBP_SafetyCharacter OtherActor)
  (Widget|RemovefromParent (stale Collision|EventActorBeginOverlap _returnvalue)))

(fn ConstructionScript)