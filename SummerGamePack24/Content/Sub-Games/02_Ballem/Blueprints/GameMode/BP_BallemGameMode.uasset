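; Game mode for the Ballem sub-game, handling the control-hint HUD, pausing, winning and level restarts.
; It creates a controls widget on BeginPlay, and custom events add, rename or remove its keyboard and controller prompts for basic, hover and path-building states.
; Winning swaps all widgets for a win screen, then after a short delay has the SGP24 game instance switch levels.
; Pausing toggles a pause widget and mouse cursor.
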(event Custom|PauseGame
  (bind _returnvalue (UserInterface|CreateWidget "/Game/Widgets/02_Ballem/Ballem_BP_PauseWidget.Ballem_BP_PauseWidget_C"))
  (UserInterface|Viewport|AddtoViewport _returnvalue 0)
  (Variables|/Script/Engine.PlayerController|SetbShowMouseCursor (Game|GetPlayerController 0) true)
  (Variables|Default|SetGamePaused true)
  (Game|SetGamePaused true))

(event Custom|UnPauseGame
  (Widget|RemovefromParent (stale Custom|PauseGame _returnvalue))
  (Variables|/Script/Engine.PlayerController|SetbShowMouseCursor (Game|GetPlayerController 0) false)
  (Variables|Default|SetGamePaused false)
  (Game|SetGamePaused false))

(event Custom|RestartLevel
  (bind _returnvalue (Game|GetCurrentLevelName true))
  (Game|OpenLevel(byName) (Utilities|String|StringToName _returnvalue)))

(event EventBeginPlay
  (bind _returnvalue (UserInterface|CreateWidget "/Game/Widgets/02_Ballem/Ballem_BP_ControlsWidget.Ballem_BP_ControlsWidget_C"))
  (bind _output_get (Variables|Default|SetControlsWidget _returnvalue))
  (UserInterface|Viewport|AddtoViewport _output_get 0))

(event EventTick
  (params (DeltaSeconds :type Float%20%28single-precision%29)))

(event EventWinGame
  (Viewport|RemoveAllWidgets)
  (bind _returnvalue (UserInterface|CreateWidget "/Game/Widgets/02_Ballem/Ballem_BP_WinGame.Ballem_BP_WinGame_C"))
  (UserInterface|Viewport|AddtoViewport _returnvalue 0)
  (Utilities|FlowControl|Delay 3.0)
  (bind _asbp_sgp24game_instance (Utilities|Casting|CastToBP_SGP24GameInstance (Game|GetGameInstance)))
  (Default|SwitchLevel _asbp_sgp24game_instance))

(event EventAddBuildControls
  ;[1 1 1] Control UI
  (Default|UpdateControlAction (Variables|Default|GetControlsWidget) "Start Build" "Continue Build")
  (Default|AddControlAction (Variables|Default|GetControlsWidget) "Confirm Build" "/Game/Widgets/Images/Xbox/XboxSeriesX_X.XboxSeriesX_X" "/Game/Widgets/Images/KeyboardMouse/Space_Key_Dark.Space_Key_Dark")
  (Default|AddControlAction (Variables|Default|GetControlsWidget) "Cancel Build" "/Game/Widgets/Images/Xbox/XboxSeriesX_B.XboxSeriesX_B" "/Game/Widgets/Images/KeyboardMouse/X_Key_Dark.X_Key_Dark"))

(event EventAddBasicControls
  ;[1 1 1] Control UI
  (Default|AddControlAction (Variables|Default|GetControlsWidget) "Start Build" "/Game/Widgets/Images/Xbox/XboxSeriesX_A.XboxSeriesX_A" "/Game/Widgets/Images/KeyboardMouse/Mouse_Left_Key_Dark.Mouse_Left_Key_Dark")
  (Default|AddControlAction (Variables|Default|GetControlsWidget) "Start Simulation" "/Game/Widgets/Images/Xbox/XboxSeriesX_Y.XboxSeriesX_Y" "/Game/Widgets/Images/KeyboardMouse/E_Key_Dark.E_Key_Dark")
  (Default|AddControlAction (Variables|Default|GetControlsWidget) "Reset Simulation" "/Game/Widgets/Images/Xbox/XboxSeriesX_View.XboxSeriesX_View" "/Game/Widgets/Images/KeyboardMouse/R_Key_Dark.R_Key_Dark")
  (Default|AddControlAction (Variables|Default|GetControlsWidget) "Move Cursor" "/Game/Widgets/Images/Xbox/XboxSeriesX_Left_Stick.XboxSeriesX_Left_Stick" "/Game/Widgets/Images/KeyboardMouse/Mouse_Simple_Key_Dark.Mouse_Simple_Key_Dark"))

(event EventRemoveBuildControls
  ;[1 1 1] Control UI
  (Default|UpdateControlAction (Variables|Default|GetControlsWidget) "Continue Build" "Start Build")
  (Default|RemoveControlAction (Variables|Default|GetControlsWidget) "Cancel Build")
  (Default|RemoveControlAction (Variables|Default|GetControlsWidget) "Confirm Build"))

(event EventAddHoverControls
  ;[1 1 1] Control UI
  (Default|AddControlAction (Variables|Default|GetControlsWidget) "Delete Path" "/Game/Widgets/Images/Xbox/XboxSeriesX_X.XboxSeriesX_X" "/Game/Widgets/Images/KeyboardMouse/Space_Key_Dark.Space_Key_Dark"))

(event EventRemoveHoverControls
  ;[1 1 1] Control UI
  (Default|RemoveControlAction (Variables|Default|GetControlsWidget) "Delete Path"))

(fn ConstructionScript)