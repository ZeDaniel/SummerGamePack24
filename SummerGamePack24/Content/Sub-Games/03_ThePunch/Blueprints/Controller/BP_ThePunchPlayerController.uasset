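; Player controller for The Punch sub-game that puts each stage's UI on screen.
; BeginPlay adds the controls widget to the viewport.
; Separate events create the accuracy score, punch score, and launch game and launch score widgets for games 2 to 4.
; The end-game event has BP_ThePunchGameMode clear the widgets, then shows the final score widget.
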(event EventBeginPlay
  (bind _returnvalue (UserInterface|CreateWidget "/Game/Widgets/03_ThePunch/BP_ControlsWidget.BP_ControlsWidget_C"))
  (UserInterface|Viewport|AddtoViewport _returnvalue 0))

(event EventTick
  (params (DeltaSeconds :type Float%20%28single-precision%29)))

(event EventRunGame2UI
  (bind _returnvalue (UserInterface|CreateWidget "/Game/Widgets/03_ThePunch/BP_AccuracyScoreWidget.BP_AccuracyScoreWidget_C"))
  (UserInterface|Viewport|AddtoViewport _returnvalue 0))

(event EventRunGame3UI
  (bind _returnvalue (UserInterface|CreateWidget "/Game/Widgets/03_ThePunch/BP_PunchScoreWidget.BP_PunchScoreWidget_C"))
  (UserInterface|Viewport|AddtoViewport _returnvalue 0))

(event EventRunGame4UI
  (bind _returnvalue (UserInterface|CreateWidget "/Game/Widgets/03_ThePunch/BP_LaunchGameWidget.BP_LaunchGameWidget_C"))
  (UserInterface|Viewport|AddtoViewport _returnvalue 0)
  (bind _returnvalue_2 (UserInterface|CreateWidget "/Game/Widgets/03_ThePunch/BP_LaunchScoreWidget1.BP_LaunchScoreWidget1_C"))
  (UserInterface|Viewport|AddtoViewport _returnvalue_2 0))

(event EventRunEndGameUI
  (bind _asbp_the_punch_game_mode (Utilities|Casting|CastToBP_ThePunchGameMode (Game|GetGameMode)))
  (Default|ClearWidgets _asbp_the_punch_game_mode)
  (bind _returnvalue (UserInterface|CreateWidget "/Game/Widgets/03_ThePunch/BP_FinalScoreWidget.BP_FinalScoreWidget_C"))
  (UserInterface|Viewport|AddtoViewport _returnvalue 0))

(fn ConstructionScript)