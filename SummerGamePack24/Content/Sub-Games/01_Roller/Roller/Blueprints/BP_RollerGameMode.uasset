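; Game mode for the Roller sub-game, handling level startup, pausing, restarting and the win screen.
; On BeginPlay it shows the HUD and intro widget with pawn input disabled, then after a short delay sets the player camera and attaches the level root to the controlled BaseLevel pawn.
; It then enables input and sets the game instance's target score from the level's target count.
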(event Custom|EndGame
  (Input|DisableInput (Game|Player|GetPlayerPawn 0) (Game|GetPlayerController 0))
  (bind _returnvalue (UserInterface|CreateWidget "/Game/Sub-Games/01_Roller/Roller/Blueprints/BP_WinWidget.BP_WinWidget_C"))
  (UserInterface|Viewport|AddtoViewport _returnvalue 0))

(event Custom|PauseGame
  (bind _returnvalue (Game|GetPlayerController 0))
  ;[1 1 1] Pause and UnPause
  (bind _returnvalue_2 (UserInterface|CreateWidget "/Game/Widgets/01_Roller/Roller_BP_PauseWidget.Roller_BP_PauseWidget_C"))
  (UserInterface|Viewport|AddtoViewport _returnvalue_2 0)
  (Variables|/Script/Engine.PlayerController|SetbShowMouseCursor _returnvalue true)
  (Variables|Default|SetGamePaused true)
  (Input|SetInputModeUIOnly _returnvalue _returnvalue_2 "DoNotLock" false)
  (Game|SetGamePaused true))

(event Custom|UnPauseGame
  (bind _returnvalue (Game|GetPlayerController 0))
  ;[1 1 1] Pause and UnPause
  (Widget|RemovefromParent (stale Custom|PauseGame _returnvalue_2))
  (Variables|/Script/Engine.PlayerController|SetbShowMouseCursor _returnvalue false)
  (Variables|Default|SetGamePaused false)
  (Input|SetInputModeGameOnly _returnvalue false)
  (Game|SetGamePaused false))

(event Custom|RestartLevel
  (bind _returnvalue (Game|GetCurrentLevelName true))
  (Game|OpenLevel(byName) (Utilities|String|StringToName _returnvalue)))

(event EventBeginPlay
  (bind _returnvalue (Game|GetPlayerController 0))
  ;[1 1 1] Handle level startup
  (bind _returnvalue_2 (UserInterface|CreateWidget "/Game/Widgets/01_Roller/Roller_BP_PlayerHud.Roller_BP_PlayerHud_C"))
  (UserInterface|Viewport|AddtoViewport _returnvalue_2 0)
  (bind _asbp_level_controller (Utilities|Casting|CastToBP_LevelController _returnvalue))
  (Input|SetInputModeGameOnly _returnvalue false)
  (Input|DisableInput (Pawn|GetControlledPawn _asbp_level_controller) 0)
  ;[1 1 1] Create level start widget
  (bind _returnvalue_3 (UserInterface|CreateWidget "/Game/Sub-Games/01_Roller/Roller/Blueprints/BP_LevelWidget.BP_LevelWidget_C"))
  (UserInterface|Viewport|AddtoViewport _returnvalue_3 0)
  (Utilities|FlowControl|Delay 3.0)
  (bind _returnvalue_4 (Actor|GetActorOfClass "/Game/Sub-Games/01_Roller/Roller/Blueprints/BP_PlayerCamera.BP_PlayerCamera_C"))
  ;[1 1 1] Add player camera to BaseLevel pawn
  (bind _asbp_base_level (Utilities|Casting|CastToBP_BaseLevel (Pawn|GetControlledPawn _asbp_level_controller)))
  (Variables|/Game/Sub-Games/01_Roller/Roller/Blueprints/BP_BaseLevel.BP_BaseLevel_C|SetPlayerCamera _asbp_base_level _returnvalue_4)
  (Game|Player|SetViewTargetwithBlend _asbp_level_controller _returnvalue_4 0.0 "VTBlend_Linear" 0.0 false)
  (bind _returnvalue_5 (Actor|GetActorOfClass "/Game/Sub-Games/01_Roller/Roller/Blueprints/BP_LevelRoot.BP_LevelRoot_C"))
  (Transformation|AttachComponentToComponent (Variables|/Script/Engine.Actor|GetRootComponent _returnvalue_5) (Variables|/Script/Engine.Actor|GetRootComponent (Pawn|GetControlledPawn _asbp_level_controller)) "" "SnapToTarget" "SnapToTarget" "KeepRelative" false)
  (Input|EnableInput (Pawn|GetControlledPawn _asbp_level_controller) _asbp_level_controller)
  ;[1 1 1] Set Target Score based on number of targets in the level
  (bind _outactors (Actor|GetAllActorsOfClass "/Game/Sub-Games/01_Roller/Roller/Blueprints/BP_Target.BP_Target_C"))
  (bind _asbp_sgp24game_instance (Utilities|Casting|CastToBP_SGP24GameInstance (Game|GetGameInstance)))
  (Default|SetTargetScore _asbp_sgp24game_instance (Utilities|Array|Length _outactors)))

(event EventTick
  (params (DeltaSeconds :type Float%20%28single-precision%29)))

(fn ConstructionScript)