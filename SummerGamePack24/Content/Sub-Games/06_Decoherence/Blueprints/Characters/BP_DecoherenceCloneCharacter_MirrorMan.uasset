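; Mirror Man clone character for the Decoherence sub-game, a variant that moves and looks with mirrored input.
; It overrides the parent's move and look input hooks, calling the parent first and then rewriting AlteredInput.
; Movement has its X axis negated, while look has both X and Y negated.
; All other behavior comes from the parent class.
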(event EventBeginPlay
  (|CallParentFunction) ; This node is disabled and will not be called.\nDrag off pins to build functionality.
)

(event Collision|EventActorBeginOverlap
  (params (OtherActor :type Actor%20Object%20Reference))
  (|CallParentFunction OtherActor) ; This node is disabled and will not be called.\nDrag off pins to build functionality.
)

(event EventTick
  (params (DeltaSeconds :type Float%20%28single-precision%29))
  (|CallParentFunction DeltaSeconds) ; This node is disabled and will not be called.\nDrag off pins to build functionality.
)

(event EventAlterMoveInput
  (params (Value :type Input%20Action%20Value%20Structure%20%28by%20ref%29))
  (|CallParentFunction Value)
  (Variables|Default|SetAlteredInput (Class|EnhancedInputLibrary|MakeInputActionValueOfType (* (.X (Class|EnhancedInputLibrary|BreakInputActionValue (Variables|Default|GetAlteredInput))) -1.0) (.Y (Class|EnhancedInputLibrary|BreakInputActionValue (Variables|Default|GetAlteredInput))) (.Z (Class|EnhancedInputLibrary|BreakInputActionValue (Variables|Default|GetAlteredInput))) "Axis2D")))

(event EventAlterLookInput
  (params (Value :type Input%20Action%20Value%20Structure%20%28by%20ref%29))
  (|CallParentFunction Value)
  (Variables|Default|SetAlteredInput (Class|EnhancedInputLibrary|MakeInputActionValueOfType (* (.X (Class|EnhancedInputLibrary|BreakInputActionValue (Variables|Default|GetAlteredInput))) -1.0) (* (.Y (Class|EnhancedInputLibrary|BreakInputActionValue (Variables|Default|GetAlteredInput))) -1.0) (.Z (Class|EnhancedInputLibrary|BreakInputActionValue (Variables|Default|GetAlteredInput))) "Axis2D")))

(fn ConstructionScript
  (|CallParentFunction))