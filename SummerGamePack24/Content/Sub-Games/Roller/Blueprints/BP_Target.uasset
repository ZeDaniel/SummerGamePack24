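; BP_Target is a one-shot target in the Roller sub-game that awards score when the player ball touches it.
; On the first Box overlap that passes a BP_PlayerBall class cast, it latches IsActivated, plays a sound and swaps the TargetPlane material to SwitchableMaterial.
; It then calls IncreaseScore on BP_RollerGameInstance, so the game instance handles the score.
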(event OnComponentBeginOverlap(Box)
  (params (OverlappedComponent :type Primitive%20Component%20Object%20Reference) (OtherActor :type Actor%20Object%20Reference) (OtherComp :type Primitive%20Component%20Object%20Reference) (OtherBodyIndex :type Integer) (bFromSweep :type Boolean) (SweepResult :type Hit%20Result%20Structure%20%28by%20ref%29))
  (if (not (Variables|Default|GetIsActivated))
    (Utilities|Casting|CastToBP_PlayerBallClass (Utilities|GetClass OtherActor))
    (Variables|Default|SetIsActivated true)
    (Audio|PlaySoundatLocation "/Game/Sounds/Magic_Missile_Launches-yoyosound_com.Magic_Missile_Launches-yoyosound_com" (Transformation|GetActorLocation) "0, 0, 0" 1.0 1.0 0.0 0 0 0 0)
    (Rendering|Material|SetMaterial (Variables|Default|GetTargetPlane) 0 (Variables|Default|GetSwitchableMaterial))
    (bind _asbp_roller_game_instance (Utilities|Casting|CastToBP_RollerGameInstance (Game|GetGameInstance)))
    (Default|IncreaseScore _asbp_roller_game_instance)))

(event EventBeginPlay)

(event EventTick
  (params (DeltaSeconds :type Float%20%28single-precision%29)))

(fn ConstructionScript)