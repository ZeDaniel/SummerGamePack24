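; Game Instance for the Roller sub-game that tracks score, target score and level progression.
; Reaching the target score notifies BP_RollerGameMode to end the game, resets the score and opens the next level after a delay.
; After the fifth level, it shows an end widget and adds a restart input mapping context to the player controller.
; RestartGame resets progress and reloads the first level.
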(event Custom|IncreaseScore
  ;[1 1 1] Increase score and check for win condition
  (Variables|Default|SetCurrentScore (+ (Variables|Default|GetCurrentScore) 1))
  (if (== (Variables|Default|GetCurrentScore) (Variables|Default|GetTargetScore))
    (bind _asbp_roller_game_mode (Utilities|Casting|CastToBP_RollerGameMode (Game|GetGameMode)))
    (Default|EndGame _asbp_roller_game_mode)
    (CallFunction|WinGame)))

(event Custom|RestartGame
  ;[1 1 1] Restart Game
  (Variables|Default|SetCurrentScore 0)
  (Variables|Default|SetCurrentLevel 0)
  (Game|OpenLevel(byObjectReference) "/Game/Sub-Games/Roller/Maps/Roller_Level01.Roller_Level01"))

(event Custom|SetTargetScore
  (params (TargetScore :type Integer))
  ;[1 1 1] Public function to set target score
  (Variables|Default|SetTargetScore TargetScore))

(event Custom|WinGame
  ;[1 1 1] Win game and transition levels
  (Variables|Default|SetCurrentScore 0)
  (Variables|Default|SetCurrentLevel (+ (Variables|Default|GetCurrentLevel) 1))
  (Utilities|FlowControl|Delay 3.0)
  (switch int (Variables|Default|GetCurrentLevel)
    (:Default
      ;[1 1 1] Handle End of Game
      (bind _returnvalue (UserInterface|CreateWidget "/Game/Sub-Games/Roller/Blueprints/BP_EndWidget.BP_EndWidget_C"))
      (UserInterface|Viewport|AddtoViewport _returnvalue 0)
      (bind _asbp_level_controller (Utilities|Casting|CastToBP_LevelController (Game|GetPlayerController 0)))
      (Input|AddMappingContext (PlayerController|LocalPlayerSubsystems|GetEnhancedInputLocalPlayerSubsystem _asbp_level_controller) "/Game/Sub-Games/Roller/Input/RestartController.RestartController" 0 "(bIgnoreAllPressedKeysUntilRelease=True,bForceImmediately=False,bNotifyUserSettings=False)"))
    (:0
      (Development|PrintString "WHAT? HOW?"))
    (:1
      (Game|OpenLevel(byObjectReference) "/Game/Sub-Games/Roller/Maps/Roller_Level02.Roller_Level02"))
    (:2
      (Game|OpenLevel(byObjectReference) "/Game/Sub-Games/Roller/Maps/Roller_Level03.Roller_Level03"))
    (:3
      (Game|OpenLevel(byObjectReference) "/Game/Sub-Games/Roller/Maps/Roller_Level04.Roller_Level04"))
    (:4
      (Game|OpenLevel(byObjectReference) "/Game/Sub-Games/Roller/Maps/Roller_Level05.Roller_Level05"))))